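; TestRoom2 is a test room Blueprint whose mesh material appears built to turn see-through when it blocks the player.
; BeginPlay puts a TestSeeThrough dynamic material instance on element 1 of the room mesh.
; PlayerHit sets an in-front-of-player flag and passes that material to ParentRayHit.
; Tick zeroes the HitPos parameter while the flag is false; only BeginPlay clears the flag here.
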(event EventBeginPlay
  (bind _returnvalue (Rendering|Material|CreateDynamicMaterialInstance (Variables|Default|Getroom_prototype_0) 1 "/Game/Materials/TestSeeThrough.TestSeeThrough" "None" :!class /Script/Engine.PrimitiveComponent))
  (bind _output_get (Variables|Default|SetThisMAT_0 _returnvalue))
  (Variables|Default|SetInFrontOfPlayer_0 false))

(event Collision|EventActorBeginOverlap
  (params (OtherActor :type Actor%20Object%20Reference)))

(event EventTick
  (params (DeltaSeconds :type Float%20%28single-precision%29))
  (if (not (Variables|Default|GetInFrontOfPlayer_0))
    (Variables|Default|SetHitLoc_0 "0, 0, 0")
    (Rendering|Material|SetVectorParameterValue (Variables|Default|GetThisMAT_0) "HitPos" (Math|Conversions|ToLinearColor(Vector) (Variables|Default|GetHitLoc_0)) :!class /Script/Engine.MaterialInstanceDynamic)))

(event EventPlayerHit
  (Variables|Default|SetInFrontOfPlayer_0 true)
  (|CallParentFunction (Variables|Default|GetThisMAT_0)))

(fn ConstructionScript)