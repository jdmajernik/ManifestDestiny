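; TestWall is a test wall actor that drives a see-through material on its Cube from a ray hit position.
; BeginPlay creates a dynamic instance of TestSeeThrough and clears InFrontOfPlayer.
; RayHit sets that flag and writes HitLoc, which this graph only ever zeroes, to the HitPos parameter.
; Tick zeroes HitPos while the flag is false; nothing here clears the flag after a hit.
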(event Custom|RayHit
  (Variables|Default|SetInFrontOfPlayer true)
  (Rendering|Material|SetVectorParameterValue (Variables|Default|GetThisMAT) "HitPos" (Math|Conversions|ToLinearColor(Vector) (Variables|Default|GetHitLoc)) :!class /Script/Engine.MaterialInstanceDynamic))

(event EventBeginPlay
  (bind _returnvalue (Rendering|Material|CreateDynamicMaterialInstance (Variables|Default|GetCube) 0 "/Game/Materials/TestSeeThrough.TestSeeThrough" "None" :!class /Script/Engine.PrimitiveComponent))
  (Variables|Default|SetThisMAT _returnvalue)
  (Variables|Default|SetInFrontOfPlayer false))

(event Collision|EventActorBeginOverlap
  (params (OtherActor :type Actor%20Object%20Reference)))

(event EventTick
  (params (DeltaSeconds :type Float%20%28single-precision%29))
  (if (not (Variables|Default|GetInFrontOfPlayer))
    (Variables|Default|SetHitLoc "0, 0, 0")
    (Rendering|Material|SetVectorParameterValue (Variables|Default|GetThisMAT) "HitPos" (Math|Conversions|ToLinearColor(Vector) (Variables|Default|GetHitLoc)) :!class /Script/Engine.MaterialInstanceDynamic)))

(fn ConstructionScript)