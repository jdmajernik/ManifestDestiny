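; TestBulletSpawn is a test weapon that can be fired, picked up and dropped.
; BeginPlay sets weapon type, range and Cube as physics parent; firing passes type, range, the FirePont transform and Bullet class to WeaponFire.
; Pickup stops physics simulation on Cube, while drop enables physics and physics-only collision on Box and prints a debug string.
; A node disabling Cube collision is unconnected and never runs.
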(event EventPickedUp
  (Physics|SetSimulatePhysics (Variables|Default|GetCube) false))

(event EventDropped
  (bind _box (Variables|Default|GetBox))
  (Collision|SetCollisionEnabled _box "PhysicsOnly")
  (Physics|SetSimulatePhysics _box true)
  (Development|PrintString "Hello"))

(event EventFireWeapon
  (CallFunction|WeaponFire (Variables|Default|GetWeaponType) (Variables|Default|GetWeaponRange) (Transformation|GetWorldTransform (Variables|Default|GetFirePont)) "/Game/Blueprints/Player/Bullet.Bullet_C"))

(event EventBeginPlay
  (Variables|Default|SetWeaponType "NewEnumerator1")
  (Variables|Default|SetWeaponRange 3.5e+02)
  (Variables|Default|SetPhysParent (Variables|Default|GetCube)))

(fn ConstructionScript)