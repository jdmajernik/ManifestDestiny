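; Test weapon Blueprint that fires from its FirePont transform and can be picked up and dropped, apparently a raycast trial.
; BeginPlay sets the weapon type, range and Cube as physics parent.
; FireWeapon passes type, range and muzzle transform to WeaponFire, which is defined outside this graph.
; PickedUp disables gravity on Cube, while Dropped enables it on Box, a different component.
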(event EventPickedUp
  (Physics|SetEnableGravity (Variables|Default|GetCube) false))

(event EventDropped
  (Physics|SetEnableGravity (Variables|Default|GetBox) true))

(event EventFireWeapon
  (CallFunction|WeaponFire (Variables|Default|GetWeaponType) (Variables|Default|GetWeaponRange) (Transformation|GetWorldTransform (Variables|Default|GetFirePont))))

(event EventBeginPlay
  (Variables|Default|SetWeaponType "NewEnumerator0")
  (Variables|Default|SetWeaponRange 3.5e+02)
  (Variables|Default|SetPhysParent (Variables|Default|GetCube)))

(fn ConstructionScript)