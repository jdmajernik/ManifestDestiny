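; Base weapon Blueprint that provides shared firing logic, with the FireWeapon event and WeaponReload left empty.
; WeaponFire switches on weapon type to RaycastFire or SpawnFire, passing Range as trace distance or bullet speed.
; RaycastFire traces forward for Pawns, ignoring the player, draws persistent debug lines and destroys the hit actor outright.
; SpawnFire spawns the given bullet class at the spawn transform but never uses the speed value.
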(event Custom|FireWeapon)

(fn ConstructionScript)

(fn WeaponFire
  (params (WeaponType :type WeaponTypes%20Enum :default "NewEnumerator0") (Range :type Float%20%28single-precision%29) (BulletSpawn :type Transform) (Bullet :type Actor%20Class%20Reference))
  (switch Utilities|FlowControl|Switch|SwitchonWeaponTypes WeaponType
    (:NewEnumerator0
      (CallFunction|RaycastFire Range BulletSpawn))
    (:NewEnumerator1
      (CallFunction|SpawnFire Range BulletSpawn Bullet))))

(fn WeaponReload)

(fn RaycastFire
  (params (FireRange :type Float%20%28single-precision%29) (FireLoc :type Transform))
  (bind (_location _rotation) (Math|Transform|BreakTransform FireLoc))
  (bind (_outhit _returnvalue) (Collision|LineTraceForObjects _location (+ _location (* (Math|Vector|GetForwardVector _rotation) FireRange)) (Utilities|Array|MakeArray "ObjectTypeQuery3") false (Utilities|Array|MakeArray (Game|GetPlayerCharacter 0)) "Persistent"))
  (if _returnvalue
    (Actor|DestroyActor (.HitActor (Collision|BreakHitResult _outhit)))))

(fn SpawnFire
  (params (bulletSpeed :type Float%20%28single-precision%29) (SpawnLoc :type Transform) (Bullet :type Actor%20Class%20Reference))
  (Game|SpawnActorfromClass Bullet SpawnLoc "AdjustIfPossibleButAlwaysSpawn" 0 0))