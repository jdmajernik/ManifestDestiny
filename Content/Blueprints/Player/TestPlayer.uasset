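; Test player for a mouse-aimed shooter that turns toward the cursor and moves relative to control yaw.
; Each tick, a camera-to-pawn trace calls PlayerHit on any blocking RoomParent wall to make it invisible.
; The action button attaches an overlapped PlayerWeapon to WeaponSocket or drops it; fire calls CodedWeapon, initially the first PlayerWeapon found.
; Pause forwards to a widget; FireBullet timer and older pickup logic are unconnected leftovers.
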(event Custom|FireBullet
  ;[1 1 1] Spawns Bullet
  (Utilities|FlowControl|Sequence
    (:then_0
      (if (> (Variables|Default|GetBulletWait) 0.1)
        (Variables|Default|SetBulletWait (- (Variables|Default|GetBulletWait) 0.1))
        (Utilities|FlowControl|Sequence
          (:then_0
            (Utilities|Time|PauseTimerbyHandle (stale _returnvalue)))
          (:then_1
            (bind _returnvalue (Utilities|Time|SetTimerbyEvent (delegate Custom|FireBullet) 0.1 true))))))
    (:then_1
      (Game|SpawnActorfromClass "/Game/Blueprints/Player/Bullet.Bullet_C" (Transformation|GetWorldTransform (Variables|Default|GetBulletSpawn)) "Undefined" 0 0))))

(event EventBeginPlay
  (Variables|/Script/Engine.PlayerController|SetbShowMouseCursor (Game|GetPlayerController 0) true)
  (Variables|Default|SetWeapon%20Equipped false)
  (bind _outactors (Actor|GetAllActorsOfClass "/Script/ManifestDestiny.PlayerWeapon"))
  (bind _output_get (Variables|Default|SetCodedWeapon (Utilities|Array|Get(acopy) _outactors)))
  (Development|PrintString (Utilities|GetDisplayName _output_get)))

(event EventTick
  (params (DeltaSeconds :type Float%20%28single-precision%29))
  (bind _returnvalue (Game|GetPlayerController 0))
  (bind _returnvalue_2 (Pawn|GetControlledPawn _returnvalue))
  (bind _returnvalue_3 (Transformation|GetActorLocation _returnvalue_2))
  ;[1 1 1] Looks at mouse
  (Transformation|SetActorRotation (Math|Interpolation|RInterpTo (Transformation|GetActorRotation _returnvalue) (Math|Rotator|MakeRotator 0.0 0.0 (.Yaw (Math|Rotator|BreakRotator (Math|Rotator|FindLookatRotation _returnvalue_3 (.Location (Collision|BreakHitResult (.HitResult (Class|PlayerController|GetHitResultUnderCursorforObjects _returnvalue (Utilities|Array|MakeArray "ObjectTypeQuery7") true)))))))) DeltaSeconds 0.0))
  ;[1 1 1] Makes Wall invisible
  (bind (_outhit _returnvalue_4) (Collision|LineTraceForObjects (Transformation|GetWorldLocation (Variables|Default|GetMainCamera)) _returnvalue_3 (Utilities|Array|MakeArray "ObjectTypeQuery1") false 0 "None"))
  (if _returnvalue_4 ; If there is a collision, try to cast
    (bind _asroom_parent (Utilities|Casting|CastToRoomParent (.HitActor (Collision|BreakHitResult _outhit)))
      (:then
        (bind _output_get (Variables|Default|SetOtherWall _asroom_parent))
        (Variables|/Script/ManifestDestiny.RoomParent|SetHitLoc _output_get (.Location (Collision|BreakHitResult _outhit)))
        (Class|RoomParent|PlayerHit _output_get)
        (Development|PrintString "HitWall"))
      (:CastFailed
        (Development|PrintString "CastFailed")))))

(event Collision|EventActorBeginOverlap
  (params (OtherActor :type Actor%20Object%20Reference))
  ;[1 1 1] Weapon Pickup
  (Development|SetHiddeninGame (Variables|Default|GetTextRender) false false))

(event Collision|EventActorEndOverlap
  (params (OtherActor :type Actor%20Object%20Reference))
  ;[1 1 1] Weapon Pickup
  (Development|SetHiddeninGame (Variables|Default|GetTextRender) true false))

(event Input|ActionEvents|InputActionFireButton
  (params (Key :type Key%20Structure))
  (bind _codedweapon (Variables|Default|GetCodedWeapon))
  (:Pressed
    (if (!= _codedweapon 0)
      (Class|PlayerWeapon|FireWeapon _codedweapon))))

(event Input|ActionEvents|InputActionActionButton
  (params (Key :type Key%20Structure))
  (:Pressed
    (if (Variables|Default|GetWeapon%20Equipped)
      (Transformation|DetachFromComponent (stale _obj) "KeepWorld" "KeepWorld" "KeepWorld" true)
      (Variables|Default|SetWeapon%20Equipped false)
      (Variables|Default|SetPlayerWeapon 0) ; Zeros out player weapon
      (Variables|Default|SetCodedWeapon 0)
      (else
        ;[1 1 1] Weapon Pickup
        (bind _asplayer_weapon (Utilities|Casting|CastToPlayerWeapon (stale Collision|EventActorBeginOverlap OtherActor)))
        (Development|PrintString "Picked up weapon")
        (bind _output_get (Variables|Default|SetCodedWeapon _asplayer_weapon))
        (Transformation|AttachComponentToComponent (Variables|/Script/Engine.Actor|GetRootComponent _output_get) (Variables|Character|GetMesh) "WeaponSocket" "SnapToTarget" "SnapToTarget" "KeepRelative" true)
        (Variables|Default|SetWeapon%20Equipped true)
        (Development|SetHiddeninGame (Variables|Default|GetTextRender) true false)))))

(event Input|ActionEvents|InputActionPauseMenu
  (params (Key :type Key%20Structure))
  (:Pressed
    (Default|PauseButtonPressed (Variables|Default|GetPauseMenuWidget))))

(event Input|AxisEvents|InputAxisHorizontal
  (params (AxisValue :type Float%20%28single-precision%29))
  ;[1 1 1] Player Movement
  (Pawn|Input|AddMovementInput (Math|Vector|GetRightVector (Math|Rotator|MakeRotator 0.0 0.0 (.Yaw (Math|Rotator|BreakRotator (Pawn|GetControlRotation :!class /Script/Engine.Pawn))))) AxisValue false))

(event Input|AxisEvents|InputAxisVertical
  (params (AxisValue :type Float%20%28single-precision%29))
  ;[1 1 1] Player Movement
  (Pawn|Input|AddMovementInput (Math|Vector|GetForwardVector (Math|Rotator|MakeRotator 0.0 0.0 (.Yaw (Math|Rotator|BreakRotator (Pawn|GetControlRotation :!class /Script/Engine.Pawn))))) AxisValue false))

(fn ConstructionScript)