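; Test enemy pawn or character that chases the player and dies when its health runs out.
; It sets Health on BeginPlay, then every Tick orders its AI controller to move toward player zero's pawn, stopping within an acceptance radius.
; The same Tick destroys the actor once Health drops below zero; nothing in this file applies damage.
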(event EventBeginPlay
  (Variables|Default|SetHealth 1e+02))

(event Collision|EventActorBeginOverlap
  (params (OtherActor :type Actor%20Object%20Reference)))

(event EventTick
  (params (DeltaSeconds :type Float%20%28single-precision%29))
  (AI|Navigation|MovetoActor (AI|GetAIController self) (Pawn|GetControlledPawn (Game|GetPlayerController 0)) 3e+02 true true true 0)
  ;[1 1 1] Actor death
  (if (< (Variables|Default|GetHealth) 0.0)
    (Actor|DestroyActor)))

(fn ConstructionScript)