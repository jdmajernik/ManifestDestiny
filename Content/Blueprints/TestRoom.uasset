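; Test room Blueprint that feeds a hit position into a see-through wall material, apparently for revealing the player.
; BeginPlay creates a dynamic TestSeeThrough material on element 1 of the RoomPrototype component.
; PlayerHit flags the room as in front of the player and calls RayHit, which writes HitLoc to the HitPos parameter.
; Tick zeroes HitLoc while unflagged, but no live path clears the flag after a hit; several leftover nodes are disconnected.
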(event EventPlayerHit
  (Variables|Default|SetInFrontOfPlayer true)
  (CallFunction|RayHit (Variables|Default|GetThisMAT)))

(event EventTick
  (params (DeltaSeconds :type Float%20%28single-precision%29))
  (if (not (Variables|Default|GetInFrontOfPlayer))
    (Variables|Default|SetHitLoc "0, 0, 0")))

(event EventBeginPlay
  (bind _returnvalue (Rendering|Material|CreateDynamicMaterialInstance (Variables|Default|Getroom_prototype) 1 "/Game/Materials/TestSeeThrough.TestSeeThrough" "None" :!class /Script/Engine.PrimitiveComponent))
  (bind _output_get (Variables|Default|SetThisMAT _returnvalue))
  (Variables|Default|SetInFrontOfPlayer false))

(fn ConstructionScript)

(fn RayHit
  (params (WallMAT :type Material%20Instance%20Dynamic%20Object%20Reference))
  (Rendering|Material|SetVectorParameterValue WallMAT "HitPos" (Math|Conversions|ToLinearColor(Vector) (Variables|Default|GetHitLoc)) :!class /Script/Engine.MaterialInstanceDynamic))